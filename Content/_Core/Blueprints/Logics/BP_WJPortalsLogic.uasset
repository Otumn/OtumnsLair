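; Logic Blueprint that creates linked pairs of WJ portals, binding to the Game Manager's portal-creation and teleport events.
; SpawnPortals spawns portals at Start and End, tracks them in CurrentActivePortals, then cross-links and enables the newest pair.
; It then teleports any valid supplied actor to the End portal.
; TPActor and DestroyPortals are empty; logic for disabling a pair and teleporting through it sits disconnected.
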(event `self.ReceiveBeginPlay`
  (`parent.ReceiveBeginPlay`))

(event `SpawnPortals`
  (params (Start :type "Vector Structure") (End :type "Vector Structure") (ActorToTp :type "Actor Object Reference"))
  (`|ExecutionSequence`
    (:`then_0`
      (bind _returnvalue (`|SpawnActorFromClass` "/Game/_Core/Blueprints/Characters/Player/WJCharacter/BP_WJPortal.BP_WJPortal_C" (`KismetMathLibrary.MakeTransform` Start) "AdjustIfPossibleButAlwaysSpawn" "OverrideRootScale" null null))
      (`KismetArrayLibrary.Array_Add` (`self.CurrentActivePortals`) _returnvalue))
    (:`then_1`
      (bind _returnvalue_2 (`|SpawnActorFromClass` "/Game/_Core/Blueprints/Characters/Player/WJCharacter/BP_WJPortal.BP_WJPortal_C" (`KismetMathLibrary.MakeTransform` End) "AdjustIfPossibleButAlwaysSpawn" "OverrideRootScale" null null))
      (`KismetArrayLibrary.Array_Add` (`self.CurrentActivePortals`) _returnvalue_2))
    (:`then_2`
      (`self.SetupTwoNewPortals`)
      (`/Engine/EditorBlueprintResources/StandardMacros.IsValid` ActorToTp
        (:`Is Valid`
          (`self.K2_SetActorLocation` ActorToTp (`self.K2_GetActorLocation` (`|GetArrayItem` (`self.CurrentActivePortals`) (- (`KismetArrayLibrary.Array_Length` (`self.CurrentActivePortals`)) 1))) false true))))))

(event `TPActor`
  (params (InPortal :type "/Game/_Core/Blueprints/Characters/Player/WJCharacter/BP_WJPortal Object Reference") (Actor :type "Actor Object Reference")))

(event `DestroyPortals`)

(fn `SetupEvents`
  (`parent.SetupEvents`)
  (add `/Game/_Core/Blueprints/BP_GameManager.WJ_CreatePortals` (`/Game/_Core/Blueprints/Libraries/BP_MainLibrary.GetGameManager`) (`|CreateDelegate` :!event `SpawnPortals`))
  (add `/Game/_Core/Blueprints/BP_GameManager.WJ_PortalTPActor` (`/Game/_Core/Blueprints/Libraries/BP_MainLibrary.GetGameManager`) (`|CreateDelegate` :!event `TPActor`)))

(fn `SetupTwoNewPortals`
  (locals (PortalA :type "/Game/_Core/Blueprints/Characters/Player/WJCharacter/BP_WJPortal Object Reference") (PortalB :type "/Game/_Core/Blueprints/Characters/Player/WJCharacter/BP_WJPortal Object Reference"))
  (`|ExecutionSequence`
    (:`then_0`
      (set `local.PortalA` (`|GetArrayItem` (`self.CurrentActivePortals`) (- (`KismetArrayLibrary.Array_Length` (`self.CurrentActivePortals`)) 2)))
      (set `local.PortalB` (`|GetArrayItem` (`self.CurrentActivePortals`) (- (`KismetArrayLibrary.Array_Length` (`self.CurrentActivePortals`)) 1))))
    (:`then_1`
      (set `/Game/_Core/Blueprints/Characters/Player/WJCharacter/BP_WJPortal.LinkedPortal` (`local.PortalB`) (`local.PortalA`))
      (set `/Game/_Core/Blueprints/Characters/Player/WJCharacter/BP_WJPortal.LinkedPortal` (`local.PortalA`) (`local.PortalB`)))
    (:`then_2`
      (`/Game/_Core/Blueprints/Characters/Player/WJCharacter/BP_WJPortal.EnablePortal` (`local.PortalB`) true)
      (`/Game/_Core/Blueprints/Characters/Player/WJCharacter/BP_WJPortal.EnablePortal` (`local.PortalA`) true))))

(fn `UserConstructionScript`
  (`parent.UserConstructionScript`))