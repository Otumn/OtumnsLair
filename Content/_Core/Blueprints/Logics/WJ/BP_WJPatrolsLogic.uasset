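; Patrol logic Blueprint that tracks the level's patrol points and resolves target positions along a given patrol.
; On BeginPlay it gathers every BP_WJPatrolPoint in the world into ScenePatrolPoints.
; GetPatrolPosition looks up a point by index in the passed patrol's own list, returning it with its location.
; If that point is occupied, the position becomes a random reachable navigation location within the supplied radius around it.
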(event `self.ReceiveBeginPlay`
  (`parent.ReceiveBeginPlay`)
  (`self.SetupPoints`))

(fn `GetPatrolPosition`
  (params (RequestedIndex :type Integer) (Patrol :type "/Game/_Core/Blueprints/Enemies/WJEnemies/BP_WJPatrol Object Reference") (PositonRadius :type "Float (double-precision)" :default 100.0))
  (returns (Position :type "Vector Structure") (targetPoint :type "/Game/_Core/Blueprints/Enemies/WJEnemies/Covers/BP_WJPatrolPoint Object Reference"))
  (bind _output (`|GetArrayItem` (`/Game/_Core/Blueprints/Enemies/WJEnemies/BP_WJPatrol.PatrolPoints` Patrol) RequestedIndex))
  (if (`/Game/_Core/Blueprints/Enemies/WJEnemies/Covers/BP_WJPatrolPoint.bOccupied?` _output)
    (return (`NavigationSystemV1.K2_GetRandomReachablePointInRadius` (`self.K2_GetActorLocation` _output) PositonRadius null null) _output)
    (else
      (return (`self.K2_GetActorLocation` _output) _output))))

(fn `SetupPoints`
  (bind _outactors (`GameplayStatics.GetAllActorsOfClass` "/Game/_Core/Blueprints/Enemies/WJEnemies/Covers/BP_WJPatrolPoint.BP_WJPatrolPoint_C"))
  (set `self.ScenePatrolPoints` _outactors))

(fn `UserConstructionScript`
  (`parent.UserConstructionScript`))