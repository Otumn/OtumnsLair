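; BP_WJShotLogic is a shot logic Blueprint that turns an intended target into a randomly deviated aim point.
; GetShotTarget rates discomfort by muzzle-to-target distance, either beyond the comfortable distance only or on both sides, with a small floor.
; That rating, Precision and MaxDeviation scale a random offset on the target, so higher Precision widens spread.
; It returns a point one unit from the muzzle along that direction, with optional debug drawing.
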(event `self.ReceiveBeginPlay`
  (`parent.ReceiveBeginPlay`))

(fn `GetShotTarget`
  (params (Muzzle :type "Vector Structure") (Target :type "Vector Structure") (ComfortableDistance :type "Float (double-precision)" :default 2500.0) (UmcomfortableRange :type "Float (double-precision)" :default 1000.0) (UncomfortableBothWays :type Boolean) (MaxDeviation :type "Float (double-precision)" :default 50.0) (Precision :type "Float (double-precision)" :default 1.0) (Debug :type Boolean))
  (returns (VectorFromStart :type "Vector Structure"))
  (locals (CalculatedVector :type "Vector Structure") (DistToTarget :type "Float (double-precision)") (ConfortResult :type "Float (double-precision)") (BaseDir :type "Vector Structure"))
  (bind _comfortabledistance (`local.ComfortableDistance`))
  (bind _comfortabledistance_2 (`local.ComfortableDistance`))
  (bind _muzzle (`local.Muzzle`))
  (bind _comfortabledistance_3 (`local.ComfortableDistance`))
  (`|ExecutionSequence`
    (:`then_0`
      (`|ExecutionSequence`
        (:`then_0`
          ;[0 1 0] Calculate ConfortResult
          (set `local.DistToTarget` (`KismetMathLibrary.FClamp` (`KismetMathLibrary.Vector_Distance` (`local.Muzzle`) (`local.Target`)) (- _comfortabledistance_3 (`local.UmcomfortableRange`)) (+ _comfortabledistance_3 (`local.UmcomfortableRange`))))
          (if (`local.UncomfortableBothWays`)
            (set `local.ConfortResult` (`KismetMathLibrary.Abs` (`KismetMathLibrary.Lerp` -1.0 1.0 (`KismetMathLibrary.NormalizeToRange` (`local.DistToTarget`) (`KismetMathLibrary.FClamp` (- _comfortabledistance_2 (`local.UmcomfortableRange`)) 0.0 _comfortabledistance_2) (+ (`local.ComfortableDistance`) (`local.UmcomfortableRange`))))))
            (else
              (set `local.ConfortResult` (`KismetMathLibrary.FClamp` (`KismetMathLibrary.NormalizeToRange` (`local.DistToTarget`) _comfortabledistance (+ _comfortabledistance (`local.UmcomfortableRange`)))))))
          (set `local.ConfortResult` (`KismetMathLibrary.FClamp` (`local.ConfortResult`) 0.02)))
        (:`then_1`
          (bind _output_get (set `local.BaseDir` (`KismetMathLibrary.Normal` (- (+ (`local.Target`) (* (`KismetMathLibrary.Normal` (`KismetMathLibrary.MakeVector` (`KismetMathLibrary.RandomFloatInRange` -1.0 1.0) (`KismetMathLibrary.RandomFloatInRange` -1.0 1.0) (`KismetMathLibrary.RandomFloatInRange` -1.0 1.0))) (`local.ConfortResult`) (`local.Precision`) (`local.MaxDeviation`))) (`local.Muzzle`)))))
          (set `local.CalculatedVector` _output_get))))
    (:`then_1`
      (if Debug
        (`KismetSystemLibrary.DrawDebugLine` _muzzle (+ _muzzle (* (`local.CalculatedVector`) (+ (`local.ComfortableDistance`) (`local.UmcomfortableRange`)))) (struct :`R` 1.0 :`G` 0.068094 :`A` 1.0) 5.0 2.0)
        (`KismetSystemLibrary.DrawDebugSphere` (+ (`local.Muzzle`) (* (`local.CalculatedVector`) (`local.ComfortableDistance`))) 10.0 8 (struct :`R` 0.081251 :`G` 1.0 :`A` 1.0) 5.0 2.0)
        (`KismetSystemLibrary.DrawDebugSphere` (+ (`local.Muzzle`) (* (`local.CalculatedVector`) (+ (`local.ComfortableDistance`) (`local.UmcomfortableRange`)))) 10.0 8 (struct :`R` 1.0 :`B` 0.193974 :`A` 1.0) 5.0 2.0)
        (if (`local.UncomfortableBothWays`)
          (`KismetSystemLibrary.DrawDebugSphere` (+ (`local.Muzzle`) (* (`local.CalculatedVector`) (- (`local.ComfortableDistance`) (`local.UmcomfortableRange`)))) 10.0 8 (struct :`R` 1.0 :`B` 0.193974 :`A` 1.0) 5.0 2.0))))
    (:`then_2`
      (return (+ (`local.Muzzle`) (`local.CalculatedVector`))))))

(fn `SetupEvents`
  (`parent.SetupEvents`))

(fn `UserConstructionScript`
  (`parent.UserConstructionScript`))