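; BP_WJDetectionLogic tracks which actors see the player and holds the WJ detection state: Neutral, Suspicious, Combat or Alert.
; Each state event sets the current state and notifies the game manager.
; The first seeing actor triggers Suspicious; losing the last one during Combat re-triggers Combat, with a cooldown timer noted as still needed.
; OnPlayerDetected is empty, and nothing here calls Neutral or Alert.
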(event `OnPlayerDetected`)

(event `AddSeeingActor`
  (params (Actor :type "Actor Object Reference"))
  (bind _seeingactors (`self.SeeingActors`))
  (`KismetArrayLibrary.Array_Add` _seeingactors Actor)
  (if (== (`KismetArrayLibrary.Array_Length` _seeingactors) 1)
    (`self.EnableSuspiciousState`)))

(event `RemoveSeeingActor`
  (params (Actor :type "Actor Object Reference"))
  (bind _seeingactors (`self.SeeingActors`))
  (`KismetArrayLibrary.Array_RemoveItem` _seeingactors Actor)
  (if (and (< (`KismetArrayLibrary.Array_Length` _seeingactors) 1) (`|EnumEquality` (`self.CurrenState`) "NewEnumerator2"))
    (`self.EnableCombatState`)))

(event `EnableNeutralState`
  (set `self.CurrenState` "NewEnumerator0")
  (`/Game/_Core/Blueprints/BP_GameManager.WJ_OnDetectNeutral` (`/Game/_Core/Blueprints/Libraries/BP_MainLibrary.GetGameManager`)))

(event `EnableSuspiciousState`
  (set `self.CurrenState` "NewEnumerator1")
  (`/Game/_Core/Blueprints/BP_GameManager.WJ_OnDetectSuspicious` (`/Game/_Core/Blueprints/Libraries/BP_MainLibrary.GetGameManager`)))

(event `EnableCombatState`
  (set `self.CurrenState` "NewEnumerator2")
  (`/Game/_Core/Blueprints/BP_GameManager.WJ_OnDetectCombat` (`/Game/_Core/Blueprints/Libraries/BP_MainLibrary.GetGameManager`)))

(event `EnableAlertState`
  (set `self.CurrenState` "NewEnumerator3")
  (`/Game/_Core/Blueprints/BP_GameManager.WJ_OnDetectAlert` (`/Game/_Core/Blueprints/Libraries/BP_MainLibrary.GetGameManager`)))

(fn `UserConstructionScript`
  (`parent.UserConstructionScript`))