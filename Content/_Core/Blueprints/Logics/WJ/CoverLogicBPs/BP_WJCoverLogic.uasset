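; Cover manager that keeps a registry of cover points and picks the best unoccupied one for an asking actor.
; GetCoverPoint scores every free point and returns the highest, drawing debug shapes for occupied points and the selected point.
; GetPointUtility sums curve-weighted distance scores with bonuses when the player is in the point's attack or cover range.
; The asker distance term measures player to asker, so it is identical for every point.
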(fn `GetCoverPoint`
  (params (AskingActor :type "Actor Object Reference"))
  (returns (Valid :type Boolean) (Cover :type "/Game/_Core/Blueprints/Enemies/WJEnemies/Covers/BP_WJCoverPoint Object Reference") (ResultUtility :type "Float (double-precision)"))
  (locals (SelectedBestValue :type "Float (double-precision)" :default -100000000.0) (CurrentTestedValue :type "Float (double-precision)") (SelectedPointIndex :type Integer) (hasValidOutput :type Boolean))
  (bind _output (`|GetArrayItem` (`self.RegisteredCoverPoints`) (`local.SelectedPointIndex`)))
  (bind _returnvalue (`self.K2_GetActorLocation` _output))
  ;[1 1 1] Maybe optimize this to only check a limited number of points around the actor
  (for (_array_element _array_index) (`self.RegisteredCoverPoints`)
    (if (not (`/Game/_Core/Blueprints/Enemies/WJEnemies/Covers/BP_WJCoverPoint.bIsOccupied?` _array_element))
      (set `local.hasValidOutput` true)
      (bind _utility (`self.GetPointUtility` _array_element AskingActor))
      (if (> _utility (`local.SelectedBestValue`))
        (set `local.SelectedBestValue` _utility)
        (set `local.SelectedPointIndex` _array_index))
      (else
        (`KismetSystemLibrary.DrawDebugSphere` (+ (`self.K2_GetActorLocation` _array_element) (0.0 0.0 450.0)) 50.0 12 (struct :`R` 0.86701 :`B` 1.0 :`A` 1.0) 0.5 5.0)
        (`KismetSystemLibrary.DrawDebugLine` (`self.K2_GetActorLocation` AskingActor) (+ (`self.K2_GetActorLocation` _array_element) (0.0 0.0 450.0)) (struct :`R` 1.0 :`B` 0.879763 :`A` 1.0) 0.5 5.0))))
  (`KismetSystemLibrary.DrawDebugLine` _returnvalue (+ _returnvalue (0.0 0.0 2500.0)) (struct :`R` 0.007687 :`G` 1.0 :`A` 1.0) 10.0 5.0)
  (return (`local.hasValidOutput`) _output (`local.SelectedBestValue`)))

(fn `GetPointUtility`
  (params (CoverPoint :type "/Game/_Core/Blueprints/Enemies/WJEnemies/Covers/BP_WJCoverPoint Object Reference") (AskingActor :type "Actor Object Reference"))
  (returns (Utility :type "Float (double-precision)"))
  (locals (Point :type "/Game/_Core/Blueprints/Enemies/WJEnemies/Covers/BP_WJCoverPoint Object Reference") (Asker :type "Actor Object Reference") (CalculatedUtility :type "Float (double-precision)"))
  (bind _output_get (set `local.Point` CoverPoint))
  (set `local.Asker` AskingActor)
  (`|ExecutionSequence`
    (:`then_0`
      (`|ExecutionSequence`
        (:`then_0`
          (set `local.CalculatedUtility` (+ (`KismetMathLibrary.Lerp` (`self.MinDistanceUtility`) (`self.MaxDistanceUtility`) (`CurveFloat.GetFloatValue` (`self.DistanceFromPlayerCurve`) (`KismetMathLibrary.NormalizeToRange` (`KismetMathLibrary.FClamp` (`KismetMathLibrary.Vector_Distance` (`self.K2_GetActorLocation` (`GameplayStatics.GetPlayerPawn` 0)) (`self.K2_GetActorLocation` (`local.Point`))) (`self.MinDistanceConsidered`) (`self.MaxDistanceConsidered`)) (`self.MinDistanceConsidered`) (`self.MaxDistanceConsidered`)))) (`local.CalculatedUtility`))))
        (:`then_1`)
        (:`then_2`
          (bind _result (`/Game/_Core/Blueprints/Enemies/WJEnemies/Covers/BP_WJCoverPoint.IsLocationInAttackRange` (`local.Point`) (`self.K2_GetActorLocation` (`GameplayStatics.GetPlayerPawn` 0))))
          (set `local.CalculatedUtility` (+ (`KismetMathLibrary.SelectFloat` (`self.InAttackRangeUtility`) 0.0 _result) (`local.CalculatedUtility`))))
        (:`then_3`
          (bind _result_2 (`/Game/_Core/Blueprints/Enemies/WJEnemies/Covers/BP_WJCoverPoint.IsLocationInCoverRange` (`local.Point`) (`self.K2_GetActorLocation` (`GameplayStatics.GetPlayerPawn` 0))))
          (set `local.CalculatedUtility` (+ (`KismetMathLibrary.SelectFloat` (`self.InCoverRangeUtility`) 0.0 _result_2) (`local.CalculatedUtility`))))
        (:`then_4`
          (set `local.CalculatedUtility` (+ (`KismetMathLibrary.Lerp` (`self.MinDistanceUtility`) (`self.MaxDistanceUtility`) (`CurveFloat.GetFloatValue` (`self.DistanceFromAskerCurve`) (`KismetMathLibrary.NormalizeToRange` (`KismetMathLibrary.FClamp` (`KismetMathLibrary.Vector_Distance` (`self.K2_GetActorLocation` (`GameplayStatics.GetPlayerPawn` 0)) (`self.K2_GetActorLocation` (`local.Asker`))) (`self.MinDistanceConsidered`) (`self.MaxDistanceConsidered`)) (`self.MinDistanceConsidered`) (`self.MaxDistanceConsidered`)))) (`local.CalculatedUtility`))))))
    (:`then_1`
      (return (`local.CalculatedUtility`)))))

(fn `RegisterPoint`
  (params (Point :type "/Game/_Core/Blueprints/Enemies/WJEnemies/Covers/BP_WJCoverPoint Object Reference"))
  (`KismetArrayLibrary.Array_Add` (`self.RegisteredCoverPoints`) Point))

(fn `UnregisterPoint`
  (params (Point :type "/Game/_Core/Blueprints/Enemies/WJEnemies/Covers/BP_WJCoverPoint Object Reference"))
  (`KismetArrayLibrary.Array_RemoveItem` (`self.RegisteredCoverPoints`) Point))

(fn `UserConstructionScript`
  (`parent.UserConstructionScript`))