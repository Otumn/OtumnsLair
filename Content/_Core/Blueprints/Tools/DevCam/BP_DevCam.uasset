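; BP_DevCam is a developer camera tool with switchable depth-of-field blur and black-and-white effects.
; ToggleBlur flips the stored focal distance on or off, and ToggleBaW flips the stored saturation between full color and grayscale.
; Both events, like the construction script, rebuild the Camera's post-process settings from those two stored values, so the effects combine.
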(event `ToggleBlur`
  (if (== (`self.CurrentFocalDistance`) 0.0)
    (set `self.CurrentFocalDistance` 11.0)
    (else
      (set `self.CurrentFocalDistance` 0.0)))
  (set `CameraComponent.PostProcessSettings` (make `PostProcessSettings` :`ColorSaturation` (`self.CurrentSaturation`) :`DepthOfFieldFocalDistance` (`self.CurrentFocalDistance`)) (`self.Camera`) :!label _label))

(event `ToggleBaW`
  (if (== (`KismetMathLibrary.BreakVector4` (`self.CurrentSaturation`)) 1.0)
    (set `self.CurrentSaturation` (`KismetMathLibrary.MakeVector4` 0.0 0.0 0.0 1.0))
    (goto _label)
    (else
      (set `self.CurrentSaturation` (`KismetMathLibrary.MakeVector4` 1.0 1.0 1.0 1.0))
      (goto _label))))

(fn `UserConstructionScript`
  (set `CameraComponent.PostProcessSettings` (make `PostProcessSettings` :`ColorSaturation` (`self.CurrentSaturation`) :`DepthOfFieldFocalDistance` (`self.CurrentFocalDistance`)) (`self.Camera`)))