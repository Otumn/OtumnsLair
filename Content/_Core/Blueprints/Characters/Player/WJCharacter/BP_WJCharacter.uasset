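; Player character Blueprint that adds gun aiming with two stances, Classic and CAR, plus input hooks for portaling.
; Holding Aim and scrolling the mouse wheel picks the stance, setting target transforms from marker components and per-stance mouse sensitivity.
; A timeline lerps GunHolder from its current transform to the target, returning to the origin saved at BeginPlay on release.
; Middle mouse requests portal search and spawn, but both actions are empty stubs.
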(event `self.ReceiveBeginPlay`
  (`parent.ReceiveBeginPlay`)
  (`self.SetupAiming`))

(event `self.ReceiveTick`
  (params (DeltaSeconds :type "Float (single-precision)"))
  (`parent.ReceiveTick` DeltaSeconds))

(event `InputAction|Aim`
  (params (Key :type "Key Structure"))
  ;[0 1 0] Aim Event
  (:`Pressed`
    (`self.RequestAim`))
  (:`Released`
    (`self.RequestUnAim`)))

(event `RequestAim`
  ;[0 1 0] Aim Requests
  (`self.DoAim`))

(event `RequestUnAim`
  ;[0 1 0] Aim Requests
  (`self.DoUnAim`))

(event `DoAim`
  ;[0 1 0] Aim actions
  (set `self.bIsAiming?` true)
  (`self.UpdateAimStanceParameters` (`self.CurrentStance`)))

(event `DoUnAim`
  ;[0 1 0] Aim actions
  (set `self.bIsAiming?` false)
  (`self.UpdateAimStanceParameters` "NewEnumerator0"))

(event `InputAction|MouseWheelUp`
  (params (Key :type "Key Structure"))
  ;[0 1 0] Aim actions
  (:`Pressed`
    (if (`self.bIsAiming?`)
      (set `self.CurrentStance` "NewEnumerator0")
      (`self.UpdateAimStanceParameters` "NewEnumerator0"))))

(event `InputAction|MouseWheelDown`
  (params (Key :type "Key Structure"))
  ;[0 1 0] Aim actions
  (:`Pressed`
    (if (`self.bIsAiming?`)
      (set `self.CurrentStance` "NewEnumerator1")
      (`self.UpdateAimStanceParameters` "NewEnumerator1"))))

(event `UpdateAimStance`
  ;[0 1 0] Aim actions
  (bind (_direction _alpha) (`Timeline|AimStanceTimeline` :!via `PlayFromStart`)
    (:`Update`
      (`SceneComponent.K2_SetRelativeLocationAndRotation` (`self.GunHolder`) (`KismetMathLibrary.VLerp` (`self.GunLastPos`) (`self.GunTargetPos`) _alpha) (`KismetMathLibrary.RLerp` (`self.GunLastRot`) (`self.GunTargetRot`) _alpha true) false false))))

(event `InputAction|MiddleMouseButton`
  (params (Key :type "Key Structure"))
  (:`Pressed`
    (`self.RequestSearchPortal`))
  (:`Released`
    (`self.RequestSpawnPortal`)))

(event `RequestSearchPortal`
  (`self.DoSearchPortal`))

(event `RequestSpawnPortal`
  (`self.DoSpawnPortal`))

(event `DoSearchPortal`)

(event `DoSpawnPortal`)

(fn `GetAimStanceTargets`
  (returns (Pos :type "Vector Structure") (Rot :type "Rotator Structure"))
  (bind _gunposaim (`self.GunPosAim`))
  (bind _gunposcar (`self.GunPosCAR`))
  (if (`self.bIsAiming?`)
    (switch `/Game/_Core/Blueprints/Characters/Player/WJCharacter/WJAimStance` (`self.CurrentStance`)
      (:`NewEnumerator0`
        (return (`SceneComponent.RelativeLocation` _gunposaim) (`SceneComponent.RelativeRotation` _gunposaim)))
      (:`NewEnumerator1`
        (return (`SceneComponent.RelativeLocation` _gunposcar) (`SceneComponent.RelativeRotation` _gunposcar))))
    (else
      (return (`self.GunOriginPos`) (`self.GunOriginRot`)))))

(fn `SetupAiming`
  (bind _gunholder (`self.GunHolder`))
  (set `self.GunOriginPos` (`SceneComponent.RelativeLocation` _gunholder))
  (set `self.GunOriginRot` (`SceneComponent.RelativeRotation` _gunholder)))

(fn `SetupTimelinesRate`
  (`parent.SetupTimelinesRate`)
  (`TimelineComponent.SetPlayRate` (`self.AimStanceTimeline`) (`self.AimStanceRate`)))

(fn `UpdateAimStanceParameters`
  (params (`New Stance` :type "/Game/_Core/Blueprints/Characters/Player/WJCharacter/WJAimStance Enum" :default "NewEnumerator0"))
  (bind (_pos _rot) (`self.GetAimStanceTargets`))
  (bind _gunholder (`self.GunHolder`))
  (bind _returnvalue (select `/Game/_Core/Blueprints/Characters/Player/WJCharacter/WJAimStance` (`self.CurrentStance`) :`NewEnumerator0` (`self.ClassicAimMouseSensi`) :`NewEnumerator1` (`self.CARAimMouseSensi`)))
  (`|ExecutionSequence`
    (:`then_0`
      (set `self.GunTargetPos` _pos)
      (set `self.GunTargetRot` _rot)
      (set `self.GunLastPos` (`SceneComponent.RelativeLocation` _gunholder))
      (set `self.GunLastRot` (`SceneComponent.RelativeRotation` _gunholder)))
    (:`then_1`
      (`self.UpdateAimStance`))
    (:`then_2`
      (if (`self.bIsAiming?`)
        (set `self.MouseTurnRate` _returnvalue)
        (set `self.MouseLookUpRate` _returnvalue)
        (else
          (set `self.MouseTurnRate` 1.0)
          (set `self.MouseLookUpRate` 1.0))))))

(fn `UserConstructionScript`
  (`parent.UserConstructionScript`))