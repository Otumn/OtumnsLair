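; Guard enemy character that provides the movement, gun and patrol-route functions for a patrolling, armed enemy.
; Movement events set the crouch flag and max walk speed, while gun events toggle weapon visibility and a one-second IsShooting flag.
; Patrol helpers pick the next point on the assigned patrol, either looping in order or randomly without repeating the current one.
; A detection gauge widget is cached on BeginPlay and turned toward the player camera every tick.
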(event `self.ReceiveBeginPlay`
  (`self.UpdateCurrentSpeed` (`self.WalkSpeed`))
  (`self.SetupDetectionGauge`))

(event `self.ReceiveTick`
  (params (DeltaSeconds :type "Float (single-precision)"))
  (set `self.DeltaTime` DeltaSeconds)
  (set `self.CurrentVelocity` (`MovementComponent.Velocity` (`self.CharacterMovement`)))
  (`self.RotateDetectionBar`))

(event `ActivateWalk`
  (set `self.isCrouched?` false)
  (`self.UpdateCurrentSpeed` (`self.WalkSpeed`)))

(event `ActivateAimWalk`
  (set `self.isCrouched?` false)
  (`self.UpdateCurrentSpeed` (`self.AimingWalkSpeed`)))

(event `ActivateRun`
  (set `self.isCrouched?` false)
  (`self.UpdateCurrentSpeed` (`self.RunSpeed`)))

(event `ActivateCrouch`
  (set `self.isCrouched?` true)
  (`self.UpdateCurrentSpeed` (`self.CrouchSpeed`)))

(event `Shoot`
  (set `self.isShooting?` true)
  (`KismetSystemLibrary.Delay` 1.0)
  (set `self.isShooting?` false))

(event `ActivateGun`
  (set `self.hasGun?` true)
  (`SceneComponent.SetVisibility` (`self.Gun`) true false))

(event `DeactivateGun`
  (set `self.hasGun?` false)
  (`SceneComponent.SetVisibility` (`self.Gun`) false false))

(fn `GetCurrentPatrolPoint`
  (returns (Point :type "/Game/_Core/Blueprints/Enemies/WJEnemies/Covers/BP_WJPatrolPoint Object Reference"))
  (return (`|GetArrayItem` (`/Game/_Core/Blueprints/Enemies/WJEnemies/BP_WJPatrol.PatrolPoints` (`self.AssignedPatrol`)) (`self.CurrentIndex`))))

(fn `RotateDetectionBar`
  (bind _detectiongauge (`self.DetectionGauge`))
  (`SceneComponent.K2_SetWorldRotation` _detectiongauge (`KismetMathLibrary.FindLookAtRotation` (`SceneComponent.K2_GetComponentLocation` _detectiongauge) (`SceneComponent.K2_GetComponentLocation` (`PlayerCameraManager.TransformComponent` (`GameplayStatics.GetPlayerCameraManager` 0)))) false false))

(fn `SetNextPatrolIndex`
  (returns (nextIndex :type Integer))
  (locals (SelectedIndex :type Integer) (Length :type Integer))
  (bind _currentindex (`self.CurrentIndex`))
  (`|ExecutionSequence`
    (:`then_0`
      (set `local.Length` (`KismetArrayLibrary.Array_Length` (`/Game/_Core/Blueprints/Enemies/WJEnemies/BP_WJPatrol.PatrolPoints` (`self.AssignedPatrol`))))
      (if (`self.bPatrolRandomly?`)
        (bind _output_get (set `local.SelectedIndex` _currentindex))
        (while (== _output_get _currentindex)
          (set `local.SelectedIndex` (`KismetMathLibrary.RandomIntegerInRange` 0 (- (`local.Length`) 1))))
        (else
          (bind _output_get_2 (set `local.SelectedIndex` (+ (`self.CurrentIndex`) 1)))
          (if (>= _output_get_2 (`local.Length`))
            (set `local.SelectedIndex` 0)))))
    (:`then_1`
      (bind _output_get_3 (set `self.NextIndex` (`local.SelectedIndex`)))
      (return _output_get_3))))

(fn `SetupDetectionGauge`
  (set `self.Gauge` (cast `/Game/_Core/Blueprints/Enemies/WJEnemies/BPW_WJDetection` (`WidgetComponent.GetUserWidgetObject` (`self.DetectionGauge`)) :!pure true)))

(fn `UpdateCurrentpatrolIndex`
  (set `self.CurrentIndex` (`self.NextIndex`)))

(fn `UpdateCurrentSpeed`
  (params (NewSpeed :type "Float (double-precision)"))
  (bind _output_get (set `CharacterMovementComponent.MaxWalkSpeed` NewSpeed (`self.CharacterMovement`)))
  (set `self.CurrentUsedSpeed` _output_get))

(fn `UserConstructionScript`)