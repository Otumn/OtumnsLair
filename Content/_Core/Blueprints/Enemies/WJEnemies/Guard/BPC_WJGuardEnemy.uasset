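; AI controller for the guard enemy, which starts its behavior tree shortly after possessing a pawn.
; Perception updates set a blackboard flag for whether the player is being detected, without yet accounting for detection-logic state.
; Helper functions access blackboard detection flags and write a normalized, scaled rotation vector.
; Cover events trigger leaving old cover and toggle cover searching off for a randomized cooldown.
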(event `self.ReceivePossess`
  (params (PossessedPawn :type "Pawn Object Reference"))
  (set `self.PossessedPawn` (cast `/Game/_Core/Blueprints/Enemies/WJEnemies/Guard/BP_WJGuardEnemy` PossessedPawn :!pure true))
  (`KismetSystemLibrary.Delay` 0.2)
  (`self.RunBehaviorTree` "/Game/_Core/Blueprints/Enemies/WJEnemies/Guard/BPBT_WJGuardEnemy.BPBT_WJGuardEnemy"))

(event `self.AIPerception.OnTargetPerceptionUpdated`
  (params (Actor :type "Actor Object Reference") (Stimulus :type "AIStimulus Structure"))
  (if (`.bSuccessfullySensed` (break `AIStimulus` Stimulus))
    ;[1 1 1] Change this to something that takes into account the detection logic state
    (`self.SetBBIsDetectingPlayer` true)
    (else
      (`self.SetBBIsDetectingPlayer` false))))

(event `UpdateOldCover`
  (`self.LeavingCover`))

(event `TriggerLookForCoverCD`
  (bind _lookforcovercdrange (`self.LookForCoverCDRange`))
  (set `self.bLookForCover?` false)
  (`KismetSystemLibrary.Delay` (+ (`self.LookForCoverCD`) (`KismetMathLibrary.RandomFloatInRange` (* _lookforcovercdrange -1.0) _lookforcovercdrange)))
  (set `self.bLookForCover?` true))

(fn `GetBBIsDetectingPlayer`
  (returns (isDetecting :type Boolean))
  (return (`BlackboardComponent.GetValueAsBool` (`AIBlueprintHelperLibrary.GetBlackboard` null) "bIsDetectingPlayer?")))

(fn `SetBBFVectorRotation`
  (params (Value :type "Vector Structure"))
  (`BlackboardComponent.SetValueAsVector` (`AIBlueprintHelperLibrary.GetBlackboard` null) "FVectorRotation" (* (`KismetMathLibrary.Normal` Value) 100.0)))

(fn `SetBBHasDetectedPlayer`
  (params (Value :type Boolean))
  (`BlackboardComponent.SetValueAsBool` (`AIBlueprintHelperLibrary.GetBlackboard` null) "bHasDetectedPlayer?" Value))

(fn `SetBBIsDetectingPlayer`
  (params (Value :type Boolean))
  (`BlackboardComponent.SetValueAsBool` (`AIBlueprintHelperLibrary.GetBlackboard` null) "bIsDetectingPlayer?" Value))

(fn `UserConstructionScript`)