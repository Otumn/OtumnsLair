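; Cover point actor for WJ enemies that registers with the WJ cover logic shortly after BeginPlay and tracks whether it is occupied.
; The construction script shapes cover and attack cones from angle and offset settings using arrows, and shifts left/right shooting openings.
; Range checks compare flattened dot products against each cone's edge arrow to test locations.
; Tick draws a red or green debug sphere above it to show occupancy.
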(event `self.ReceiveBeginPlay`
  (`KismetSystemLibrary.Delay` 0.2)
  (`/Game/_Core/Blueprints/Logics/WJ/CoverLogicBPs/BP_WJCoverLogic.RegisterPoint` (`/Game/_Core/Blueprints/Libraries/BP_MainLibrary.GetWJCoverLogic`) self))

(event `SetOccupant`
  (set `self.bIsOccupied?` true))

(event `RemoveOccupant`
  (set `self.bIsOccupied?` false))

(event `self.ReceiveTick`
  (params (DeltaSeconds :type "Float (single-precision)"))
  (bind _returnvalue (+ (`self.K2_GetActorLocation`) (0.0 0.0 300.0)))
  (if (`self.bIsOccupied?`)
    (`KismetSystemLibrary.DrawDebugSphere` _returnvalue 100.0 12 (struct :`R` 1.0 :`B` 0.004751 :`A` 1.0) 0.0 2.0)
    (else
      (`KismetSystemLibrary.DrawDebugSphere` _returnvalue 100.0 12 (struct :`R` 0.145227 :`G` 1.0 :`A` 1.0) 0.0 2.0))))

(fn `IsLocationInAttackRange`
  (params (TestedLocation :type "Vector Structure"))
  (returns (Result :type Boolean) (Margin :type "Float (double-precision)"))
  (bind _attackangleparent (`self.AttackAngleParent`))
  (bind _returnvalue (`KismetMathLibrary.MakeVector` (.x (`SceneComponent.GetForwardVector` _attackangleparent)) (.y (`SceneComponent.GetForwardVector` _attackangleparent))))
  (return (> (`KismetMathLibrary.Dot_VectorVector` _returnvalue (`KismetMathLibrary.Normal` (`KismetMathLibrary.MakeVector` (.x (- TestedLocation (`SceneComponent.K2_GetComponentLocation` _attackangleparent))) (.y (- TestedLocation (`SceneComponent.K2_GetComponentLocation` _attackangleparent)))))) (`KismetMathLibrary.Dot_VectorVector` _returnvalue (`KismetMathLibrary.MakeVector` (.x (`SceneComponent.GetForwardVector` (`self.PosAttRangeArrow`))) (.y (`SceneComponent.GetForwardVector` (`self.PosAttRangeArrow`)))))) 0.0))

(fn `IsLocationInCoverRange`
  (params (TestedLocation :type "Vector Structure"))
  (returns (Result :type Boolean) (Margin :type "Float (double-precision)"))
  (bind _coveredangleparent (`self.CoveredAngleParent`))
  (bind _returnvalue (`KismetMathLibrary.MakeVector` (.x (`SceneComponent.GetForwardVector` _coveredangleparent)) (.y (`SceneComponent.GetForwardVector` _coveredangleparent))))
  (return (> (`KismetMathLibrary.Dot_VectorVector` _returnvalue (`KismetMathLibrary.Normal` (`KismetMathLibrary.MakeVector` (.x (- TestedLocation (`SceneComponent.K2_GetComponentLocation` _coveredangleparent))) (.y (- TestedLocation (`SceneComponent.K2_GetComponentLocation` _coveredangleparent)))))) (`KismetMathLibrary.Dot_VectorVector` _returnvalue (`KismetMathLibrary.MakeVector` (.x (`SceneComponent.GetForwardVector` (`self.PosCoverRangeArrow`))) (.y (`SceneComponent.GetForwardVector` (`self.PosCoverRangeArrow`)))))) 0.0))

(fn `UserConstructionScript`
  (`|ExecutionSequence`
    (:`then_0`
      (`SceneComponent.K2_SetRelativeRotation` (`self.PosCoverRangeArrow`) (`KismetMathLibrary.MakeRotator` 0.0 0.0 (`self.CoverAngleRange`)) false false)
      (`SceneComponent.K2_SetRelativeRotation` (`self.NegCoverRangeArrow`) (`KismetMathLibrary.MakeRotator` 0.0 0.0 (* (`self.CoverAngleRange`) -1.0)) false false)
      (`SceneComponent.K2_SetRelativeRotation` (`self.CoveredAngleParent`) (`KismetMathLibrary.MakeRotator` 0.0 0.0 (`self.CoverAngleOffset`)) false false)
      (`SceneComponent.K2_SetRelativeRotation` (`self.PosAttRangeArrow`) (`KismetMathLibrary.MakeRotator` 0.0 0.0 (`self.AttackAngleRange`)) false false)
      (`SceneComponent.K2_SetRelativeRotation` (`self.NegAttRangeArrow`) (`KismetMathLibrary.MakeRotator` 0.0 0.0 (* (`self.AttackAngleRange`) -1.0)) false false)
      (`SceneComponent.K2_SetRelativeRotation` (`self.AttackAngleParent`) (`KismetMathLibrary.MakeRotator` 0.0 0.0 (`self.AttackAngleOffset`)) false false))
    (:`then_1`
      (set `ArrowComponent.ArrowLength` (`KismetMathLibrary.SelectFloat` (`self.Debug_SightRange`) 80.0 (`self.DEBUG`)) (`self.PosCoverRangeArrow`))
      (set `ArrowComponent.ArrowLength` (`KismetMathLibrary.SelectFloat` (`self.Debug_SightRange`) 80.0 (`self.DEBUG`)) (`self.FowardArrow`))
      (set `ArrowComponent.ArrowLength` (`KismetMathLibrary.SelectFloat` (`self.Debug_SightRange`) 80.0 (`self.DEBUG`)) (`self.NegCoverRangeArrow`))
      (set `ArrowComponent.ArrowLength` (`KismetMathLibrary.SelectFloat` (`self.Debug_SightRange`) 80.0 (`self.DEBUG`)) (`self.PosAttRangeArrow`))
      (set `ArrowComponent.ArrowLength` (`KismetMathLibrary.SelectFloat` (`self.Debug_SightRange`) 80.0 (`self.DEBUG`)) (`self.NegAttRangeArrow`)))
    (:`then_2`
      (for _array_element (`self.CoverOpenings`)
        (bind (_opening _offset) (break `/Game/_Core/Blueprints/Enemies/WJEnemies/Covers/BPS_CoverOpeningsInfos` _array_element))
        (switch `/Game/_Core/Blueprints/Enemies/WJEnemies/Covers/BPE_CoverPointOpenings` _opening
          (:`NewEnumerator1`
            (`SceneComponent.K2_AddLocalOffset` (`self.ShootRightOpening`) (`KismetMathLibrary.MakeVector` 0.0 _offset) false false))
          (:`NewEnumerator2`
            (`SceneComponent.K2_AddLocalOffset` (`self.ShootLeftOpening`) (`KismetMathLibrary.MakeVector` 0.0 (* _offset -1.0)) false false)))))))