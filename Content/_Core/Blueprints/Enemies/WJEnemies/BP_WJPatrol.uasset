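; BP_WJPatrol is a patrol path actor for WJ enemies that holds an array of patrol point actors.
; Its construction script rebuilds a spline with linear segments through the points' world locations, tinted with a debug color to visualize the route in the editor.
; GetPoint returns the patrol point at a given index.
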(fn `DrawDebugPath`
  (bind _debugcolor (`self.DebugColor`))
  (`|ExecutionSequence`
    (:`then_0`
      (`SplineComponent.ClearSplinePoints` (`self.Spline`) true))
    (:`then_1`
      (for (_array_element _array_index) (`self.PatrolPoints`)
        (`SplineComponent.AddSplinePoint` (`self.Spline`) (`self.K2_GetActorLocation` _array_element) "World" true)
        (`SplineComponent.SetSplinePointType` (`self.Spline`) _array_index "Linear" true)))
    (:`then_2`
      (`SplineComponent.SetSelectedSplineSegmentColor` (`self.Spline`) _debugcolor)
      (`SplineComponent.SetUnselectedSplineSegmentColor` (`self.Spline`) _debugcolor))))

(fn `GetPoint`
  (params (Index :type Integer))
  (returns (Point :type "/Game/_Core/Blueprints/Enemies/WJEnemies/Covers/BP_WJPatrolPoint Object Reference"))
  (return (`|GetArrayItem` (`self.PatrolPoints`) Index)))

(fn `UserConstructionScript`
  (`self.DrawDebugPath`))